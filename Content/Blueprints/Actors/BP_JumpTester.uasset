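; BP_JumpTester is an actor that previews a jump arc with debug spheres from its construction script.
; It derives vertical launch speed from gravity and max height, using take-off speed horizontally along world X.
; Fixed time steps apply quadratic air drag and gravity, storing points and coloring ascent blue, descent to start height yellow.
; The event graph holds only disconnected experiments, including timed movement and capsule-trace surface sliding.
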(event `self.ReceiveBeginPlay`)

(event `CustomEvent`
  (`self.K2_SetActorLocation` (+ (`self.K2_GetActorLocation`) (`KismetMathLibrary.MakeVector` 23.0))))

(event `self.ReceiveTick`
  (params (DeltaSeconds :type "Float (single-precision)")))

(fn `Calculate Shift`
  (params (_velocity :type Integer))
  (returns (_shift :type Integer))
  (return (`KismetMathLibrary.Round` (* _velocity (`self.timeStep`)))))

(fn `Draw Jump`
  (params (_velocityX :type "Integer (by ref)") (_velocityY :type "Integer (by ref)") (_currentLocation :type "Vector Structure (by ref)") (_debugSphereColor :type "LinearColor Structure"))
  (`self.UpdateVirtualLocation&Velocity` _velocityX _velocityY _currentLocation)
  (`KismetArrayLibrary.Array_Add` (`self.jumpLocations`) _currentLocation)
  (`KismetSystemLibrary.DrawDebugSphere` _currentLocation 5.0 2 _debugSphereColor 10.0))

(fn `GetJumpVelocityImpulse`
  (params (_gravityAcceleration :type Integer) (_jumpMaxHeight :type Integer))
  (returns (_velocityImpulse :type Integer))
  (return (`KismetMathLibrary.Round` (`KismetMathLibrary.Sqrt` (`KismetMathLibrary.Conv_IntToDouble` (* (* _gravityAcceleration _jumpMaxHeight) 2))))))

(fn `Update Drag Force on Virtual Velocity`
  (params (inVelocity :type Integer) (drag :type "Float (double-precision)") (`applyGravity?` :type Boolean))
  (returns (outVelocity :type Integer))
  (locals (NewLocalVar :type Boolean) (dragDecel :type "Float (double-precision)") (inVel :type Integer))
  (bind _output_get (set `local.inVel` inVelocity))
  (bind _returnvalue (`KismetMathLibrary.Conv_IntToDouble` _output_get))
  (set `local.dragDecel` (* (* (* (`KismetMathLibrary.Square` (/ _returnvalue 100.0)) (* (`KismetMathLibrary.SignOfFloat` _returnvalue) -1)) 100.0) drag))
  (if `applyGravity?`
    (bind _output_get_2 (set `local.dragDecel` (+ (`local.dragDecel`) (* (`self.gravityAceleration`) -1.0))))
    (bind _output_get_3 (set `local.inVel` (`KismetMathLibrary.Round` (+ (`local.inVel`) (* _output_get_2 (`self.timeStep`))))))
    (return _output_get_3)
    (else
      (bind _output_get_4 (set `local.inVel` (`KismetMathLibrary.Round` (+ (`local.inVel`) (* (`local.dragDecel`) (`self.timeStep`))))))
      (return _output_get_4))))

(fn `UpdateVirtualLocation&Velocity`
  (params (_velocityX :type "Integer (by ref)") (_velocityY :type "Integer (by ref)") (_currentLoc :type "Vector Structure (by ref)"))
  (locals (currentLoc :type "Vector Structure") (velX :type Integer) (velY :type Integer))
  (set `local.velX` _velocityX)
  (set `local.velY` _velocityY)
  (set `local.currentLoc` _currentLoc)
  (`|VariableSetRef` _currentLoc (+ (`local.currentLoc`) (`KismetMathLibrary.MakeVector` (`KismetMathLibrary.Conv_IntToDouble` (`self.Calculate Shift` (`local.velX`))) 0.0 (`KismetMathLibrary.Conv_IntToDouble` (`self.Calculate Shift` (`local.velY`))))))
  (`|VariableSetRef` _velocityX (`self.Update Drag Force on Virtual Velocity` (`local.velX`) (`self.airDrag`)))
  (`|VariableSetRef` _velocityY (`self.Update Drag Force on Virtual Velocity` (`local.velY`) (`self.airDrag`) true)))

(fn `UserConstructionScript`
  (locals (velocityX :type Integer) (velocityY :type Integer) (startingLocation :type "Vector Structure") (currentLocation :type "Vector Structure") (movementVector :type "Vector Structure"))
  (bind (_currentlocation_x _currentlocation_y _currentlocation_z) (`KismetMathLibrary.BreakVector` (`local.currentLocation`)))
  (bind (_startinglocation_x _startinglocation_y _startinglocation_z) (`KismetMathLibrary.BreakVector` (`local.startingLocation`)))
  (`|ExecutionSequence`
    (:`then_0`
      (set `local.velocityX` (`self.jumpTakeOffSpeed`))
      (set `local.velocityY` (`self.GetJumpVelocityImpulse` (`self.gravityAceleration`) (`self.jumpMaxHieght`)))
      (bind _output_get (set `local.startingLocation` (`self.K2_GetActorLocation`)))
      (set `local.currentLocation` _output_get)
      (`KismetArrayLibrary.Array_Clear` (`self.jumpLocations`)))
    (:`then_1`
      (while (or (> (`local.velocityY`) 0) (> (`KismetArrayLibrary.Array_Length` (`self.jumpLocations`)) 500))
        (`self.Draw Jump` (`local.velocityX`) (`local.velocityY`) (`local.currentLocation`) (struct :`G` 0.15 :`B` 1.0 :`A` 1.0)))
      (while (> _currentlocation_z _startinglocation_z)
        (`self.Draw Jump` (`local.velocityX`) (`local.velocityY`) (`local.currentLocation`) (struct :`R` 1.0 :`G` 1.0 :`A` 1.0))))))