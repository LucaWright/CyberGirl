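; Blueprint function library of kinematic helpers for gravity and velocity updates.
; CalculateVelocityDelta multiplies acceleration by a time step capped at a very small maximum.
; ApplyGravity adds that delta as downward acceleration; its AirDrag and Area2D inputs are unused, so drag is absent.
; UpdateVelocity uses the delta's magnitude as a constant interpolation step toward a directional target speed.
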(fn `Apply Gravity`
  (params (_gravity :type "Float (double-precision)") (_velocityOnNegativeGravityDirection :type "Float (double-precision)") (_airDrag :type "Float (double-precision)") (_area2D :type "Float (double-precision)") (_timeStep :type "Float (double-precision)" :default 0.02) (_context :type "Object Object Reference"))
  (returns (_updatedVelocity :type "Float (double-precision)"))
  (return (+ _velocityOnNegativeGravityDirection (`self.CalculateVelocityDelta` (+ (* (`KismetMathLibrary.Abs` _gravity) -1.0) 0.0) _timeStep _context))))

(fn `CalculateVelocityDelta`
  (params (acceleration :type "Float (double-precision)") (timeStep :type "Float (double-precision)" :default 0.02))
  (returns (`Return Value` :type "Float (double-precision)"))
  (return (* acceleration (`KismetMathLibrary.FMin` timeStep 0.001))))

(fn `Test`
  (params (NewParam :type "Float (double-precision)"))
  (returns (NewParam1 :type "Float (double-precision)"))
  (return (* NewParam 0.0)))

(fn `UpdateVelocity`
  (params (_acceleration :type "Float (double-precision)") (_currentSpeed :type "Float (double-precision)") (_targetSpeed :type "Float (double-precision)") (_direction :type "Float (double-precision)") (_timeStep :type "Float (double-precision)" :default 0.02) (_context :type "Object Object Reference"))
  (returns (_updatedVelocity :type "Float (double-precision)"))
  (return (`KismetMathLibrary.FInterpTo_Constant` _currentSpeed (* _targetSpeed _direction) 1.0 (`KismetMathLibrary.Abs` (`self.CalculateVelocityDelta` _acceleration _timeStep _context)))))